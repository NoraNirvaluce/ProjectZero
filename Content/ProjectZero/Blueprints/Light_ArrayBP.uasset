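; Light_ArrayBP is a construction-script Blueprint that lays out copies of one static mesh in a flat grid.
; It adds X minus Y instances to a HierarchicalInstancedStaticMesh component, using division and modulo by Y to derive each row and column.
; SpaceX and SpaceY set the spacing, with rotation and scale left at defaults, and the StaticMesh variable is reassigned on every loop pass.
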(fn ConstructionScript
  (bind _y (Variables|Default|GetY))
  (bind _hierarchicalinstancedstaticmesh (Variables|Default|GetHierarchicalInstancedStaticMesh))
  ;[1 1 1] ArrayMesh
  (for _index (range 0 (- (- (Variables|Default|GetX) (Variables|Default|GetY)) 1))
    (Components|InstancedStaticMesh|AddInstance _hierarchicalinstancedstaticmesh (Math|Transform|MakeTransform (Math|Vector|MakeVector (* (/ _index _y) (Variables|Default|GetSpaceX)) (* (Math|Integer|%(Integer) _index _y) (Variables|Default|GetSpaceY)) 0.0)))
    (Components|StaticMesh|SetStaticMesh _hierarchicalinstancedstaticmesh (Variables|Default|GetStaticMesh))))